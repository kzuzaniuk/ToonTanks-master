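; BP_GameModeBase is the game mode that shows start and end screens and handles level progression.
; GameStart creates a start widget and passes it the start delay.
; GameOver shows WBP_GameEnd with the result and kill count, then waits through a fixed delay.
; A win opens Level2 from Main or Level3 from any other level, while a loss reloads the current level by name.
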(event `self.GameStart`
  (bind _returnvalue (`|CreateWidget` "/Game/Blueprints/Widgets/WBP_GameStart.WBP_GameStart_C"))
  (`/Game/Blueprints/Widgets/WBP_GameStart.SetStartDelay` _returnvalue (`self.StartDelay`))
  (`UserWidget.AddToViewport` _returnvalue 0))

(event `self.GameOver`
  (params (PlayerWon :type Boolean))
  (bind _returnvalue (`|CreateWidget` "/Game/Blueprints/Widgets/WBP_GameEnd.WBP_GameEnd_C"))
  (`/Game/Blueprints/Widgets/WBP_GameEnd.SetPlayerWon` _returnvalue PlayerWon)
  (`/Game/Blueprints/Widgets/WBP_GameEnd.SetKillCount` _returnvalue (`self.KillCount`))
  (`UserWidget.AddToViewport` _returnvalue 0)
  (`KismetSystemLibrary.Delay` 15.0)
  (if (== true PlayerWon)
    (bind _returnvalue_2 (`GameplayStatics.GetCurrentLevelName` true))
    (if (`KismetStringLibrary.EqualEqual_StrStr` "Main" _returnvalue_2)
      (`GameplayStatics.OpenLevel` "Level2")
      (else
        (`GameplayStatics.OpenLevel` "Level3")))
    (else
      (bind _returnvalue_3 (`GameplayStatics.GetCurrentLevelName` true))
      (`GameplayStatics.OpenLevel` (`KismetStringLibrary.Conv_StringToName` _returnvalue_3)))))

(fn `UserConstructionScript`)